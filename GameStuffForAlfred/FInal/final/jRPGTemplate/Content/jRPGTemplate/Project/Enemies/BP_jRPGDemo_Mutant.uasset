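; Mutant enemy for the jRPG template demo that makes a simple attack on a random player character during its AI turn.
; PerformActionbyAI shows a battle tooltip, ends its turn through the battle manager, then uses timed delays around the attack montage, stat-based damage with crit and impact particle before resuming battle.
; The construction script tints the mannequin body with a dynamic material and attaches a skeletal mesh to the weapon socket.
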(event `self.PerformActionByAI`
  (bind _battlemanagerreference (`self.BattleManagerReference`))
  (bind _playercharacters (`/Game/jRPGTemplate/Blueprints/Components/AC_jRPG_BattleManager.PlayerCharacters` (`self.BattleManagerReference`)))
  (bind _characterstats (`/Game/jRPGTemplate/Blueprints/Components/AC_jRPG_CharacterBattleStats.CharacterStats` (`self.AC_jRPG_CharacterStats`)))
  (`/Game/jRPGTemplate/Blueprints/Components/AC_jRPG_BattleManager.ShowBattleTooltip` _battlemanagerreference (`|FormatText` "{name} attacks" (`/Game/jRPGTemplate/Blueprints/Components/AC_jRPG_CharacterBattleStats.CharacterDisplayName` (`self.AC_jRPG_CharacterStats`))))
  (`/Game/jRPGTemplate/Blueprints/Components/AC_jRPG_BattleManager.EndCharacterTurn` _battlemanagerreference 1000.0)
  (`KismetSystemLibrary.Delay` 0.25)
  (`self.PlayAnimMontage` "/Game/jRPGTemplate/Project/Mannequin/Animations/AM_SimpleAttack.AM_SimpleAttack")
  (`KismetSystemLibrary.Delay` 0.3)
  (bind _output_get (set `self.Targeted` (`|GetArrayItem` _playercharacters (`KismetMathLibrary.RandomIntegerInRange` 0 (- (`KismetArrayLibrary.Array_Length` _playercharacters) 1)))))
  (`/Game/jRPGTemplate/Blueprints/Components/AC_jRPG_CharacterBattleStats.ReceiveDamage` (`/Game/jRPGTemplate/Blueprints/Basics/BP_jRPG_Character_Battle_Base.AC_jRPG_CharacterStats` _output_get) (`BlueprintMapLibrary.Map_Find` _characterstats "NewEnumerator3") (`BlueprintMapLibrary.Map_Find` _characterstats "NewEnumerator5") (`BlueprintMapLibrary.Map_Find` _characterstats "NewEnumerator6"))
  (`GameplayStatics.SpawnEmitterAtLocation` "/Game/jRPGTemplate/Project/VFX/Particles/Impact/P_Impact_Generic.P_Impact_Generic" (`self.K2_GetActorLocation` _output_get))
  (`KismetSystemLibrary.Delay` 1.0)
  (`/Game/jRPGTemplate/Blueprints/Components/AC_jRPG_BattleManager.ResumeBattle` (`self.BattleManagerReference`)))

(fn `UserConstructionScript`
  (`parent.UserConstructionScript`)
  (bind _returnvalue (`PrimitiveComponent.CreateDynamicMaterialInstance` (`self.Mesh`) 0 "/Game/jRPGTemplate/Project/Mannequin/Character/Materials/M_UE4Man_Body.M_UE4Man_Body" "None"))
  (`MaterialInstanceDynamic.SetVectorParameterValue` _returnvalue "BodyColor" (struct :`R` 0.0625 :`G` 0.007555 :`A` 1.0))
  (bind _returnvalue_2 (`AddComponent|NODE_AddSkeletalMeshComponent-0`))
  (`SceneComponent.K2_AttachToComponent` _returnvalue_2 (`self.Mesh`) "weapon_socket" "SnapToTarget" "SnapToTarget" "SnapToTarget" true))