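; Interactable door for the jRPG template, a child interaction object that toggles open and closed when a world character interacts with it.
; Each interaction flips the stored interaction state and swaps the door's static mesh between open and closed versions, with no animation.
; When the saved interaction state loads, the matching mesh is applied so the door keeps its last state.
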(event `/Game/jRPGTemplate/Blueprints/Interfaces/BPI_Interaction.OnObjectInteractionStateLoaded`
  (params (InteractionState :type Boolean))
  ;[1 1 1] Set proper mesh when object interaction state is loaded.
  (if InteractionState
    (`StaticMeshComponent.SetStaticMesh` (`self.DoorMesh`) "/Game/jRPGTemplate/Project/InteractableObjects/Meshes/SM_Door_Open.SM_Door_Open")
    (else
      (`StaticMeshComponent.SetStaticMesh` (`self.DoorMesh`) "/Game/jRPGTemplate/Project/InteractableObjects/Meshes/SM_Door_Closed.SM_Door_Closed"))))

(event `/Game/jRPGTemplate/Blueprints/Interfaces/BPI_Interaction.OnInteractionRequested`
  (params (InteractingWorldCharacter :type "/Game/jRPGTemplate/Blueprints/Basics/BP_jRPG_Character_World Object Reference"))
  ;[1 1 1] Interact with door.
  (`/Engine/EditorBlueprintResources/StandardMacros.IsValid` InteractingWorldCharacter
    (:`Is Valid`
      (if (`self.GetObjectInteractionState`)
        (`self.SetObjectInteractionState` false) ; Mark door as closed.
        (`StaticMeshComponent.SetStaticMesh` (`self.DoorMesh`) "/Game/jRPGTemplate/Project/InteractableObjects/Meshes/SM_Door_Closed.SM_Door_Closed") ; Change mesh to closed door.
        (else
          (`self.SetObjectInteractionState` true) ; Mark door as open.
          (`StaticMeshComponent.SetStaticMesh` (`self.DoorMesh`) "/Game/jRPGTemplate/Project/InteractableObjects/Meshes/SM_Door_Open.SM_Door_Open") ; Change mesh to open door.
        )))))

(fn `UserConstructionScript`
  (`parent.UserConstructionScript`))