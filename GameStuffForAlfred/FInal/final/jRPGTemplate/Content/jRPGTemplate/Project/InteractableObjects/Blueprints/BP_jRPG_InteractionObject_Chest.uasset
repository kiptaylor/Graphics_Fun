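; Lootable chest interaction object for the jRPG template that grants its items to the player once.
; On first interaction it adds each ItemsInChest entry to the player's inventory manager and shows a pop-up built from DT_jRPG_Items display names and amounts.
; It then sets its interaction state to opened, so later attempts only report an empty chest.
; The open or closed mesh follows that state, including when it is loaded.
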(event `/Game/jRPGTemplate/Blueprints/Interfaces/BPI_Interaction.OnObjectInteractionStateLoaded`
  (params (InteractionState :type Boolean))
  ;[1 1 1] Set proper mesh when object interaction state is loaded.
  (if InteractionState
    (`StaticMeshComponent.SetStaticMesh` (`self.ChestMesh`) "/Game/jRPGTemplate/Project/InteractableObjects/Meshes/SM_Chest_Open.SM_Chest_Open")
    (else
      (`StaticMeshComponent.SetStaticMesh` (`self.ChestMesh`) "/Game/jRPGTemplate/Project/InteractableObjects/Meshes/SM_Chest_Closed.SM_Chest_Closed"))))

(event `/Game/jRPGTemplate/Blueprints/Interfaces/BPI_Interaction.OnInteractionRequested`
  (params (InteractingWorldCharacter :type "/Game/jRPGTemplate/Blueprints/Basics/BP_jRPG_Character_World Object Reference"))
  (bind _playercontroller (`/Game/jRPGTemplate/Blueprints/Basics/BP_jRPG_Character_World.PlayerController` InteractingWorldCharacter))
  ;[1 1 1] Interact with chest.
  (`/Engine/EditorBlueprintResources/StandardMacros.IsValid` InteractingWorldCharacter
    (:`Is Valid`
      (if (`self.GetObjectInteractionState`)
        (`/Game/jRPGTemplate/Blueprints/Basics/BP_jRPG_Controller_World.ShowInteractionPopUp` _playercontroller "Chest is empty.")
        (else
          (`self.AddItemsFromChestToInventory` (`/Game/jRPGTemplate/Blueprints/Basics/BP_jRPG_Controller_World.AC_jRPG_InventoryManager` _playercontroller)) ; Add items to player inventory.
          (`/Game/jRPGTemplate/Blueprints/Basics/BP_jRPG_Controller_World.ShowInteractionPopUp` _playercontroller (`self.ConstructInteractionPopUpText`)) ; Show pop up with looted items.
          (`self.SetObjectInteractionState` true) ; Mark chest as opened.
          (`StaticMeshComponent.SetStaticMesh` (`self.ChestMesh`) "/Game/jRPGTemplate/Project/InteractableObjects/Meshes/SM_Chest_Open.SM_Chest_Open") ; Change mesh to open chest.
        )))))

(fn `AddItemsFromChestToInventory`
  (params (InventoryManager :type "/Game/jRPGTemplate/Blueprints/Components/AC_jRPG_InventoryManager Object Reference"))
  (bind _keys (`BlueprintMapLibrary.Map_Keys` (`self.ItemsInChest`)))
  (for _array_element _keys
    (`/Game/jRPGTemplate/Blueprints/Components/AC_jRPG_InventoryManager.AddItemToInventory` InventoryManager _array_element (`BlueprintMapLibrary.Map_Find` (`self.ItemsInChest`) _array_element))))

(fn `ConstructInteractionPopUpText`
  (returns (PopUpText :type Text))
  (locals (PopUpTextLOCAL :type Text :default "NSLOCTEXT(\"\", \"99F4AF35493BF814F6FF20A85C30B9C4\", \"You have gained\")"))
  (bind _itemsinchest (`self.ItemsInChest`))
  (bind _keys (`BlueprintMapLibrary.Map_Keys` _itemsinchest))
  (for _array_element _keys
    (bind _returnvalue (`|GetDataTableRow` "/Game/jRPGTemplate/Datatables/DT_jRPG_Items.DT_jRPG_Items" _array_element)
      (:`then`
        (set `local.PopUpTextLOCAL` (`|FormatText` "{current text}{row to add}" (`local.PopUpTextLOCAL`) (`|FormatText` " \n{item name} x {amount}" (`.ItemDisplayName_29_41C0C54E4A55598869C84CA3B5B5DECA` (break `/Game/jRPGTemplate/Structures/S_jRPG_Item_StaticData` _returnvalue)) (`BlueprintMapLibrary.Map_Find` _itemsinchest _array_element)))))))
  (set `local.PopUpTextLOCAL` (`|FormatText` "{current text}." (`local.PopUpTextLOCAL`))) ; Add period at the end of the info.
  (return (`local.PopUpTextLOCAL`)))

(fn `UserConstructionScript`
  (`parent.UserConstructionScript`))