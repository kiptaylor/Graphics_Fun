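; Argon, a mage player character in the jRPG template demo, built on a parent class that supplies stats and battle hooks.
; Attack, item, magic, move and Deathblow events show a battle tooltip, end the turn through the battle manager, then play mage montages, varied for some spells.
; Death and resurrection toggle the Dead flag and notify the manager.
; Impact montages, body tint and staff attachment are unwired, so never run.
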(event `self.OnDeath`
  (set `/Game/jRPGTemplate/Blueprints/Components/AC_jRPG_CharacterBattleStats.Defending` false (`self.AC_jRPG_CharacterStats`))
  (set `self.Dead?` true)
  (`self.StopAnimMontage` (`self.GetCurrentMontage`))
  (bind _battlemanagerreference (`self.BattleManagerReference`)
    (:`then`
      (`/Game/jRPGTemplate/Blueprints/Components/AC_jRPG_BattleManager.OnPlayerCharacterKilled` _battlemanagerreference self))
    (:`else`)))

(event `self.OnDamageReceived`
  (params (Damage :type "Float (single-precision)") (`Critical?` :type Boolean))
  (`parent.OnDamageReceived` Damage `Critical?`)
  (if (`/Game/jRPGTemplate/Blueprints/Components/AC_jRPG_CharacterBattleStats.Defending` (`self.AC_jRPG_CharacterStats`))
    _))

(event `self.OnResurrected`
  (params (HealAmount :type "Float (single-precision)"))
  (`parent.OnResurrected` HealAmount)
  (set `self.Dead?` false)
  (bind _battlemanagerreference (`self.BattleManagerReference`)
    (:`then`
      (`/Game/jRPGTemplate/Blueprints/Components/AC_jRPG_BattleManager.OnPlayerCharacterResurrected` _battlemanagerreference self))
    (:`else`)))

(event `self.ExecuteAttackAction`
  (bind _battlemanagerreference (`self.BattleManagerReference`)
    (:`then`
      (`/Game/jRPGTemplate/Blueprints/Components/AC_jRPG_BattleManager.ShowBattleTooltip` _battlemanagerreference (`|FormatText` "{name} attacks" (`/Game/jRPGTemplate/Blueprints/Components/AC_jRPG_CharacterBattleStats.CharacterDisplayName` (`self.AC_jRPG_CharacterStats`))))
      (`/Game/jRPGTemplate/Blueprints/Components/AC_jRPG_BattleManager.EndCharacterTurn` (`self.BattleManagerReference`) 1000.0)
      (`self.PlayAnimMontage` "/Game/jRPGTemplate/Project/GenericCharacter/Animations/Mage/AM_GenChar_Mage_Attack_01.AM_GenChar_Mage_Attack_01"))
    (:`else`)))

(event `self.ExecuteItemAction`
  (params (ItemName :type Name))
  (switch `name` ItemName
    (:`Default`
      (bind _battlemanagerreference (`self.BattleManagerReference`)
        (:`then`
          (`/Game/jRPGTemplate/Blueprints/Components/AC_jRPG_BattleManager.ShowBattleTooltip` _battlemanagerreference (`|FormatText` "{char name} uses {item name}" (`/Game/jRPGTemplate/Blueprints/Components/AC_jRPG_CharacterBattleStats.CharacterDisplayName` (`self.AC_jRPG_CharacterStats`)) (`/Game/jRPGTemplate/Blueprints/Basics/FL_jRPG_CustomFunctionLibrary.GetItemDisplayName` ItemName)))
          (`/Game/jRPGTemplate/Blueprints/Components/AC_jRPG_BattleManager.EndCharacterTurn` (`self.BattleManagerReference`) 1000.0)
          (`self.PlayAnimMontage` "/Game/jRPGTemplate/Project/GenericCharacter/Animations/Mage/AM_GenChar_Mage_UseItem.AM_GenChar_Mage_UseItem"))
        (:`else`)))))

(event `self.ExecuteMagicAction`
  (params (MagicName :type Name))
  (`parent.ExecuteMagicAction` MagicName)
  (bind _battlemanagerreference (`self.BattleManagerReference`)
    (:`then`
      (`/Game/jRPGTemplate/Blueprints/Components/AC_jRPG_BattleManager.ShowBattleTooltip` _battlemanagerreference (`|FormatText` "{char name} casts {spell name}" (`/Game/jRPGTemplate/Blueprints/Components/AC_jRPG_CharacterBattleStats.CharacterDisplayName` (`self.AC_jRPG_CharacterStats`)) (`/Game/jRPGTemplate/Blueprints/Basics/FL_jRPG_CustomFunctionLibrary.GetActionDisplayName` MagicName)))
      (`/Game/jRPGTemplate/Blueprints/Components/AC_jRPG_BattleManager.EndCharacterTurn` (`self.BattleManagerReference`) 1000.0)
      (switch `name` MagicName
        (:`Default`
          (`self.PlayAnimMontage` "/Game/jRPGTemplate/Project/GenericCharacter/Animations/Mage/AM_GenChar_Mage_CastSpell.AM_GenChar_Mage_CastSpell"))
        (:`Magic_Fireball`
          (`self.PlayAnimMontage` "/Game/jRPGTemplate/Project/GenericCharacter/Animations/Mage/AM_GenChar_Mage_Attack_01.AM_GenChar_Mage_Attack_01"))
        (:`Magic_Thunder`
          (`self.PlayAnimMontage` "/Game/jRPGTemplate/Project/GenericCharacter/Animations/Mage/AM_GenChar_Mage_Attack_02.AM_GenChar_Mage_Attack_02"))))
    (:`else`)))

(event `self.ExecuteMoveAction`
  (params (MoveName :type Name))
  (`parent.ExecuteMoveAction` MoveName)
  (bind _battlemanagerreference (`self.BattleManagerReference`)
    (:`then`
      (`/Game/jRPGTemplate/Blueprints/Components/AC_jRPG_BattleManager.ShowBattleTooltip` _battlemanagerreference (`|FormatText` "{char name} performs {move name}" (`/Game/jRPGTemplate/Blueprints/Components/AC_jRPG_CharacterBattleStats.CharacterDisplayName` (`self.AC_jRPG_CharacterStats`)) (`/Game/jRPGTemplate/Blueprints/Basics/FL_jRPG_CustomFunctionLibrary.GetActionDisplayName` MoveName)))
      (`/Game/jRPGTemplate/Blueprints/Components/AC_jRPG_BattleManager.EndCharacterTurn` (`self.BattleManagerReference`) 1000.0)
      (switch `name` MoveName
        (:`Default`
          (`self.PlayAnimMontage` "/Game/jRPGTemplate/Project/GenericCharacter/Animations/Mage/AM_GenChar_Mage_Attack_03.AM_GenChar_Mage_Attack_03"))))
    (:`else`)))

(event `self.ExecuteDeathblowAction`
  (bind _battlemanagerreference (`self.BattleManagerReference`)
    (:`then`
      (`/Game/jRPGTemplate/Blueprints/Components/AC_jRPG_BattleManager.ShowBattleTooltip` _battlemanagerreference (`|FormatText` "{name} uses Deathblow!" (`/Game/jRPGTemplate/Blueprints/Components/AC_jRPG_CharacterBattleStats.CharacterDisplayName` (`self.AC_jRPG_CharacterStats`))))
      (`/Game/jRPGTemplate/Blueprints/Components/AC_jRPG_BattleManager.EndCharacterTurn` (`self.BattleManagerReference`) 1000.0)
      (`self.PlayAnimMontage` "/Game/jRPGTemplate/Project/GenericCharacter/Animations/Mage/AM_GenChar_Mage_Deathblow.AM_GenChar_Mage_Deathblow"))
    (:`else`)))

(fn `UserConstructionScript`)