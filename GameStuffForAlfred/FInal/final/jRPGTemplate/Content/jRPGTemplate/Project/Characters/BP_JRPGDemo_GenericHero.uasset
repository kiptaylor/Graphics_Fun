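; BP_JRPGDemo_GenericHero is a demo hero character for the jRPG template's battle system.
; On death it flags itself dead and notifies the BattleManager; damage and resurrection spawn damage or healing pop-up actors.
; Magic and move actions only pay their HP and MP costs here, looked up from the player controller's ActionsManager and deducted through the character stats component.
; The body-colour material setup in the construction script is disconnected.
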(event `/Game/jRPGTemplate/Blueprints/Interfaces/BPI_BattleCommunication.OnDeath`
  (set `self.Dead?` true)
  (bind _battlemanagerreference (`self.BattleManagerReference`)
    (:`then`
      (`/Game/jRPGTemplate/Blueprints/Components/AC_jRPG_BattleManager.OnPlayerCharacterKilled` _battlemanagerreference self))
    (:`else`)))

(event `/Game/jRPGTemplate/Blueprints/Interfaces/BPI_BattleCommunication.OnDamageReceived`
  (params (Damage :type "Float (single-precision)") (`Critical?` :type Boolean))
  (`|SpawnActorFromClass` "/Game/jRPGTemplate/Blueprints/Other/Battle/BP_jRPG_DamagePopUp.BP_jRPG_DamagePopUp_C" (`KismetMathLibrary.MakeTransform` (`self.K2_GetActorLocation`)) "Undefined" "OverrideRootScale" null Damage `Critical?` false false false null))

(event `/Game/jRPGTemplate/Blueprints/Interfaces/BPI_BattleCommunication.OnResurrected`
  (params (HealAmount :type "Float (single-precision)"))
  (`|SpawnActorFromClass` "/Game/jRPGTemplate/Blueprints/Other/Battle/BP_jRPG_DamagePopUp.BP_jRPG_DamagePopUp_C" (`self.GetTransform`) "Undefined" "OverrideRootScale" null HealAmount false true false false null) ; Spawns healing pop up
)

(event `self.ExecuteMagicAction`
  (params (MagicName :type Name))
  (bind _ac_jrpg_characterstats (`self.AC_jRPG_CharacterStats`))
  (bind (_costhp _costmp) (`/Game/jRPGTemplate/Blueprints/Components/AC_jRPG_ActionsManager.GetActionCost` (`self.GetComponentByClass` (`GameplayStatics.GetPlayerController` 0) "/Game/jRPGTemplate/Blueprints/Components/AC_jRPG_ActionsManager.AC_jRPG_ActionsManager_C") MagicName))
  (`/Game/jRPGTemplate/Blueprints/Components/AC_jRPG_CharacterBattleStats.ReduceHP` _ac_jrpg_characterstats _costhp)
  (`/Game/jRPGTemplate/Blueprints/Components/AC_jRPG_CharacterBattleStats.ReduceMP` _ac_jrpg_characterstats _costmp))

(event `self.ExecuteMoveAction`
  (params (MoveName :type Name))
  (bind _ac_jrpg_characterstats (`self.AC_jRPG_CharacterStats`))
  (bind (_costhp _costmp) (`/Game/jRPGTemplate/Blueprints/Components/AC_jRPG_ActionsManager.GetActionCost` (`self.GetComponentByClass` (`GameplayStatics.GetPlayerController` 0) "/Game/jRPGTemplate/Blueprints/Components/AC_jRPG_ActionsManager.AC_jRPG_ActionsManager_C") MoveName))
  (`/Game/jRPGTemplate/Blueprints/Components/AC_jRPG_CharacterBattleStats.ReduceHP` _ac_jrpg_characterstats _costhp)
  (`/Game/jRPGTemplate/Blueprints/Components/AC_jRPG_CharacterBattleStats.ReduceMP` _ac_jrpg_characterstats _costmp))

(fn `UserConstructionScript`
  (`parent.UserConstructionScript`))